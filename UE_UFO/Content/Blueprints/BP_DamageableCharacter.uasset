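; BP_DamageableCharacter is a character with hit points that takes damage and can spawn bullets.
; AnyDamage subtracts damage from Hp, then destroys the actor at zero or below, or prints the remaining Hp otherwise.
; A SpawnBullet event spawns an actor at the BulletSpawn component's location using the character's rotation, with itself as owner; the spawned class is not shown.
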(event Custom|SpawnBullet
  (Game|SpawnActorfromClass "/Game/Blueprints/BP_Bullet.BP_Bullet_C" (Math|Transform|MakeTransform (Transformation|GetWorldLocation (Variables|Default|GetBulletSpawn)) (Transformation|GetActorRotation) "1.000000,1.000000,1.000000") "Undefined" "MultiplyWithRoot" self 0))

(event Game|Damage|EventAnyDamage
  (params (Damage :type Float%20%28single-precision%29) (DamageType :type Damage%20Type%20Object%20Reference) (InstigatedBy :type Controller%20Object%20Reference) (DamageCauser :type Actor%20Object%20Reference))
  (bind _output_get (Variables|Default|SetHp (- (Variables|Default|GetHp) Damage)))
  (if (<= _output_get 0.0)
    (Actor|DestroyActor)
    (else
      (Development|PrintString (Utilities|String|ToString(Float) _output_get)))))

(fn ConstructionScript)