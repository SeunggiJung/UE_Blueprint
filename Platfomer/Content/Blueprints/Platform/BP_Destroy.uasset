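; BP_Destroy is a platform actor that sinks and disappears once the player touches it.
; BeginPlay stores the start location, and a BP_Player overlap on the Trigger component plays a timeline.
; The timeline's alpha lerps the actor straight down from that location without sweeping, then the actor destroys itself when the timeline finishes.
; A SetLifeSpan node is left unconnected and never runs.
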(event OnComponentBeginOverlap(Trigger)
  (params (OverlappedComponent :type Primitive%20Component%20Object%20Reference) (OtherActor :type Actor%20Object%20Reference) (OtherComp :type Primitive%20Component%20Object%20Reference) (OtherBodyIndex :type Integer) (bFromSweep :type Boolean) (SweepResult :type Hit%20Result%20Structure%20%28by%20ref%29))
  (Utilities|Casting|CastToBP_Player OtherActor)
  (bind _alpha (Timeline|타임라인 Play)
    (:Update
      (Transformation|SetActorLocation (+ (Variables|Default|GetStartLoc) (Math|Vector|MakeVector 0.0 0.0 (Math|Float|Lerp 0.0 -2e+02 _alpha))) false false))
    (:Finished
      (Actor|DestroyActor))))

(event EventBeginPlay
  (Variables|Default|SetStartLoc (Transformation|GetActorLocation)))

(event EventTick
  (params (DeltaSeconds :type Float%20%28single-precision%29)))

(fn ConstructionScript
  (|CallParentFunction))