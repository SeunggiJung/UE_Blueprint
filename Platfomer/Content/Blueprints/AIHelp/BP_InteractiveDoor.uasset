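; BP_InteractiveDoor is a door that shows an interaction prompt to a nearby BP_Player and slides upward once opened.
; Overlapping the box creates the InteractWidgetClass widget on screen, and leaving removes it.
; Interact only sets IsOpen, after which Tick uses VInterpTo to ease the actor toward a point above its starting location, with no logic to close it again.
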(event OnComponentBeginOverlap(Box)
  (params (OverlappedComponent :type Primitive%20Component%20Object%20Reference) (OtherActor :type Actor%20Object%20Reference) (OtherComp :type Primitive%20Component%20Object%20Reference) (OtherBodyIndex :type Integer) (bFromSweep :type Boolean) (SweepResult :type Hit%20Result%20Structure%20%28by%20ref%29))
  (Utilities|Casting|CastToBP_Player OtherActor)
  (bind _returnvalue (UserInterface|CreateWidget (Variables|Default|GetInteractWidgetClass)))
  (bind _output_get (Variables|Default|SetInteractWidgetInstance _returnvalue))
  (UserInterface|Viewport|AddtoViewport _output_get 0))

(event OnComponentEndOverlap(Box)
  (params (OverlappedComponent :type Primitive%20Component%20Object%20Reference) (OtherActor :type Actor%20Object%20Reference) (OtherComp :type Primitive%20Component%20Object%20Reference) (OtherBodyIndex :type Integer))
  (Utilities|Casting|CastToBP_Player OtherActor)
  (Widget|RemovefromParent (Variables|Default|GetInteractWidgetInstance))
  (Variables|Default|SetInteractWidgetInstance 0))

(event EventBeginPlay
  (Variables|Default|SetStart%20Loc (Transformation|GetActorLocation)))

(event EventTick
  (params (DeltaSeconds :type Float%20%28single-precision%29))
  (if (Variables|Default|GetbIsOpen)
    (Transformation|SetActorLocation (Math|Interpolation|VInterpTo (Transformation|GetActorLocation) (+ (Variables|Default|GetStart%20Loc) "0.000000,0.000000,500.000000") DeltaSeconds 0.5) false false)))

(fn ConstructionScript)

(fn Interact
  (Variables|Default|SetbIsOpen true))